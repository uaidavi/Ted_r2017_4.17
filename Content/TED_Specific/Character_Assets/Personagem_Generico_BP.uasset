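; Generic player character Blueprint handling movement, spring-arm camera, multi-jump, montage attack combos, health and death.
; Axis input turns or strafes depending on velocity, and camera pitch is clamped.
; Two attack inputs open combos, then pick follow-up montages by previous attack and reset-timer elapsed time; block and riposte are empty stubs.
; Lethal damage stores the damage type's respawn delay, then the server unpossesses and destroys the character.
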(event Custom|DeathEvent
  ;[1 0.1638 0.124] Executa a morte do personagem, independente do motivo
  (Variables|HealthVars|SetCurHealth 0)
  (bind _is_dead (Gameplay_Functions|DeathBehavior))
  (if _is_dead
    (Actor|DestroyActor) ; A destruíção do ator ativa a notificação do controlador para permitir o respawn
    (else
      (Development|PrintString "Can't kill that which must still live"))))

(event EventBeginPlay)

(event EventActorBeginOverlap
  (params (OtherActor :type Actor%20Object%20Reference)))

(event EventTick
  (params (DeltaSeconds :type Float%20%28single-precision%29))
  ;[1 0.1638 0.124] Testa constantemente se o HP do personagem chegou a 0
  (Variables|Default|SetPassedTime DeltaSeconds))

(event EventOnLanded
  (params (Hit :type Hit%20Result%20Structure%20%28by%20ref%29))
  ;[0.2531 0.3765 1] Funções de movimento
  (Variables|MovementVars|SetJumpNum 1))

(event Game|Damage|EventAnyDamage
  (params (Damage :type Float%20%28single-precision%29) (DamageType :type Damage%20Type%20Object%20Reference) (InstigatedBy :type Controller%20Object%20Reference) (DamageCauser :type Actor%20Object%20Reference))
  ;[1 0.1638 0.124] Aplica dano ao personagem de fato
  (bind _output_get (Variables|HealthVars|SetCurHealth (- (Variables|HealthVars|GetCurHealth) (Math|Float|Floor Damage))))
  (if (<= _output_get 0)
    (Variables|Default|SetRespawnDelayTime (Variables|/Game/TED_Specific/Gameplay_Blueprints/BaseDamageType.BaseDamageType_C|GetRespawnTime (.AsBase%20Damage%20Type (Utilities|Casting|CastToBaseDamageType DamageType))))
    (CallFunction|DeathEvent)))

(event Input|ActionEvents|InputActionJump_Inp
  (params (Key :type Key%20Structure))
  ;[0.2531 0.3765 1] Funções de movimento
  (:Pressed
    (CallFunction|DoubleJump)))

(event Input|ActionEvents|InputActionAtk_1_Inp
  (params (Key :type Key%20Structure))
  ;[0.08351 1 0.1068] Funções de Ataque
  (:Pressed
    (switch int (Variables|AttackVars|GetComboNumb)
      (:0
        (Combat|Atk1Call)
        (bind _returnvalue (Utilities|Time|SetTimerbyFunctionName 0 "ResetComboFN" 6.0)))
      (:1
        (if (>= (Class|KismetSystemLibrary|GetTimerElapsedTimeHandle _returnvalue) 1.4)
          (switch int (Variables|AttackVars|GetWhatPreviousAtk)
            (:0
              (Combat|Atk11Call (Class|KismetSystemLibrary|GetTimerElapsedTimeHandle _returnvalue)))
            (:1
              (Combat|Atk21Call (Class|KismetSystemLibrary|GetTimerElapsedTimeHandle (stale _returnvalue))))))))))

(event Input|ActionEvents|InputActionAtk_2_Inp
  (params (Key :type Key%20Structure))
  ;[0.08351 1 0.1068] Funções de Ataque
  (:Pressed
    (switch int (Variables|AttackVars|GetComboNumb)
      (:0
        (Combat|Atk2Call)
        (bind _returnvalue (Utilities|Time|SetTimerbyFunctionName 0 "ResetComboFN" 6.0)))
      (:1
        (if (>= (Class|KismetSystemLibrary|GetTimerElapsedTimeHandle _returnvalue) 1.4)
          (switch int (Variables|AttackVars|GetWhatPreviousAtk)
            (:0
              (Combat|Atk12Call (Class|KismetSystemLibrary|GetTimerElapsedTimeHandle _returnvalue)))
            (:1
              (Combat|Atk22Call (Class|KismetSystemLibrary|GetTimerElapsedTimeHandle (stale _returnvalue))))))))))

(event Input|AxisEvents|InputAxisRunForward
  (params (AxisValue :type Float%20%28single-precision%29))
  ;[0.2531 0.3765 1] Funções de movimento
  (CallFunction|RunFWD/BWD AxisValue))

(event Input|AxisEvents|InputAxisPanVert
  (params (AxisValue :type Float%20%28single-precision%29))
  ;[0.2531 0.3765 1] Funções de movimento
  (CallFunction|CamRotationY AxisValue))

(event Input|AxisEvents|InputAxisPanHor
  (params (AxisValue :type Float%20%28single-precision%29))
  ;[0.2531 0.3765 1] Funções de movimento
  (CallFunction|CamRotationX AxisValue))

(event Input|AxisEvents|InputAxisMoveTurnSide
  (params (AxisValue :type Float%20%28single-precision%29))
  ;[0.2531 0.3765 1] Funções de movimento
  (CallFunction|SidewaysMove/Turn AxisValue))

(fn ConstructionScript)

(fn Atk2Call
  (Variables|AttackVars|SetWhatPreviousAtk 2)
  (Animation|Montage|MontagePlay (Components|SkeletalMesh|GetAnimInstance (Variables|Character|GetMesh)) "/Game/TED_Specific/Character_Assets/Proxy_Ted/Mont_Combo_2.Mont_Combo_2" 1.0 "MontageLength" 0.0 true)
  (Math|Integer|IncrementInt (Variables|AttackVars|GetComboNumb)))

(fn BlockCall)

(fn RiposteCall)

(fn Atk1Call
  (Variables|AttackVars|SetCanAttack false)
  (Variables|AttackVars|SetWhatPreviousAtk 1)
  (Animation|Montage|MontagePlay (Components|SkeletalMesh|GetAnimInstance (Variables|Character|GetMesh)) "/Game/TED_Specific/Character_Assets/Proxy_Ted/Mont_Combo_1.Mont_Combo_1" 1.0 "MontageLength" 0.0 true)
  (Math|Integer|IncrementInt (Variables|AttackVars|GetComboNumb)))

(fn OnRepHealthDe-Buff)

(fn DeathBehavior
  ;[1 0.1638 0.124] Como deve agir ao morrer
  (Networking|SwitchHasAuthority
    (:Authority
      (Utilities|TestIsDead ; Teste de redundância, garante que o personagem está morto.
        (:Is_Dead
          ;;[1 1 1] Retira a posse do controlador sobre o personagem se ele estiver morto.
          (Development|PrintString "Morri")
          (bind _asplayer_controller_bp (Utilities|Casting|CastToPlayer_Controller_BP (Pawn|GetController))
            (:then
              (Pawn|UnPossess _asplayer_controller_bp))
            (:CastFailed
              (Development|PrintString "Death Cast fail" true true "(R=1.000000,G=0.742836,B=0.027617,A=1.000000)" 2e+01)))
          (return true) ; Retorna com um aviso de que o personagem está morto para continuar o processo de morte
        )
        (:Is_Alive
          _)))
    (:Remote
      _))
  (return false))

(fn StringTest
  (for _array_element 0
    (Development|PrintString _array_element true true "(R=0.000000,G=0.660000,B=1.000000,A=1.000000)" 5.0)))

(fn DoubleJump
  (if (< (Variables|MovementVars|GetJumpNum) 3)
    (if (== (Variables|MovementVars|GetJumpNum) 1)
      (Variables|Default|SetJump_Height 2.5e+03)
      (else
        (Variables|Default|SetJump_Height 1.5e+03)))
    (Character|LaunchCharacter (Math|Vector|MakeVector 0.0 0.0 (Variables|Default|GetJump_Height)) false true)
    (Variables|Default|SetJump_Height 5e+03)
    (Math|Integer|IncrementInt (Variables|MovementVars|GetJumpNum))))

(fn RunFWD/BWD
  (params (A :type Float%20%28single-precision%29))
  ;[0.2531 0.3765 1] Função de movimentação frente/costas
  (if (not (Variables|Default|GetIsIncapacitated))
    (Pawn|Input|AddMovementInput (Math|Vector|GetForwardVector (Math|Rotator|MakeRotator 0.0 0.0 (.Yaw (Math|Rotator|BreakRotator (Pawn|GetControlRotation (Game|GetPlayerController 0) :!class /Script/Engine.Controller))))) (* A 1.0) true)))

(fn CamRotationX
  (params (NewParam :type Float%20%28single-precision%29))
  ;[0.2531 0.3765 1] Rotação da camera na horizontal
  ;;[1 1 1] Adiciona rotação somente na câmera se o personagem estiver parado e retorna.
  (Transformation|AddRelativeRotation (Variables|Default|GetSpringArm) (Math|Rotator|MakeRotator 0.0 0.0 NewParam) false false)
  (if (Utilities|VelocityTest)
    ;;[0.2531 0.3765 1] Adiciona rotação também sobre o personagem se ele estiver em movimento.
    (Pawn|Input|AddControllerYawInput (* NewParam 0.4))
    (return)
    (else
      (return))))

(fn CamRotationY
  (params (InputAxis :type Float%20%28single-precision%29))
  (bind (_toohigh _toolow) (Utilities|CameraRotTest))
  (bind _springarm (Variables|Default|GetSpringArm))
  (bind _springarm_2 (Variables|Default|GetSpringArm))
  (bind _relativerotation (Variables|/Script/Engine.SceneComponent|GetRelativeRotation _springarm_2))
  (bind _relativerotation_2 (Variables|/Script/Engine.SceneComponent|GetRelativeRotation _springarm))
  ;[0.2531 0.3765 1] Rotação da câmera na vertical
  (if _toohigh ; Testa se o ângulo está "muito alto"
    ;;[1 1 1] Trava a rotação da câmera se a rotação dela em "y" for maior que -50º
    (Transformation|SetRelativeRotation _springarm (Math|Rotator|MakeRotator (.roll _relativerotation_2) -47.99 (.yaw _relativerotation_2)) false false)
    (elif _toolow ; Testa se o ângulo está "muito baixo"
      ;;[1 1 1] Trava a rotação da câmera se a rotação dela em "y" for menor que -50º
      (Transformation|SetRelativeRotation _springarm_2 (Math|Rotator|MakeRotator (.roll _relativerotation) 47.99 (.yaw _relativerotation)) false false)
      (else
        ;;[1 1 1] Adiciona rotação em "y" se o valor for válido.
        (Transformation|AddRelativeRotation (Variables|Default|GetSpringArm) (Math|Rotator|MakeRotator 0.0 InputAxis 0.0) false false))))
  (return))

(fn SidewaysMove/Turn
  (params (NewParam :type Float%20%28single-precision%29))
  ;[0.2531 0.3765 1] Move ou gira o personagem lateralmente
  (if (Utilities|VelocityTest) ; Testa se o personagem está parado para\ndeterminar se ele irá rotacionar ou se mover\nlateralmente.
    ;;[1 1 1] Caso o personagem esteja já em movimento é adicionado
    ;; movimento lateral.
    (Pawn|Input|AddMovementInput (Math|Vector|GetRightVector (Math|Rotator|MakeRotator 0.0 0.0 (.Yaw (Math|Rotator|BreakRotator (Pawn|GetControlRotation (Game|GetPlayerController 0) :!class /Script/Engine.Controller))))) NewParam false)
    (else
      ;;[1 1 1] Caso o personagem esteja parado ele apenas rotaciona no lugar
      (Pawn|Input|AddControllerYawInput NewParam)))
  (return))

(fn Atk11Call
  (params (CD_TimeComparison :type Float%20%28single-precision%29))
  (if (>= CD_TimeComparison 2.0)
    (Variables|AttackVars|SetWhatPreviousAtk 1)
    (Animation|Montage|MontagePlay (Components|SkeletalMesh|GetAnimInstance (Variables|Character|GetMesh)) "/Game/TED_Specific/Character_Assets/Proxy_Ted/Mont_Combo_1_1.Mont_Combo_1_1" 1.0 "MontageLength" 0.0 true)
    (Combat|ResetComboFN)))

(fn Atk12Call
  (params (CD_TimeComparison :type Float%20%28single-precision%29))
  (if (>= CD_TimeComparison 3.0)
    (Variables|AttackVars|SetWhatPreviousAtk 2)
    (Animation|Montage|MontagePlay (Components|SkeletalMesh|GetAnimInstance (Variables|Character|GetMesh)) "/Game/TED_Specific/Character_Assets/Proxy_Ted/Mont_Combo_1_2.Mont_Combo_1_2" 1.0 "MontageLength" 0.0 true)
    (Combat|ResetComboFN)))

(fn Atk21Call
  (params (CD_TimeComparison :type Float%20%28single-precision%29))
  (if (>= CD_TimeComparison 3.0)
    (Variables|AttackVars|SetWhatPreviousAtk 1)
    (Animation|Montage|MontagePlay (Components|SkeletalMesh|GetAnimInstance (Variables|Character|GetMesh)) "/Game/TED_Specific/Character_Assets/Proxy_Ted/Mont_Combo_2_1.Mont_Combo_2_1" 1.0 "MontageLength" 0.0 true)
    (Combat|ResetComboFN)))

(fn Atk22Call
  (params (CD_TimeComparison :type Float%20%28single-precision%29))
  (if (>= CD_TimeComparison 3.0)
    (Variables|AttackVars|SetWhatPreviousAtk 2)
    (Animation|Montage|MontagePlay (Components|SkeletalMesh|GetAnimInstance (Variables|Character|GetMesh)) "/Game/TED_Specific/Character_Assets/Proxy_Ted/Mont_Combo_2_2.Mont_Combo_2_2" 1.0 "MontageLength" 0.0 true)
    (Combat|ResetComboFN)))

(fn ResetComboFN
  (Development|PrintString "ResettingCombo" true true "(R=0.000000,G=0.660000,B=1.000000,A=1.000000)" 1e+01)
  (Variables|AttackVars|SetIsNewCombo true)
  (Variables|AttackVars|SetComboNumb 0))
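; Player controller that handles character selection, respawning and control-rotation alignment for Personagem_Generico_BP pawns.
; It binds to pawn destruction, waits the character's respawn delay, then possesses the pawn GeneralRules returns for the selected character.
; Tick watches for movement starting, then a timeline lerps control rotation from the character's rotation to its spring arm's relative rotation.
; Menu acceptance is forwarded to GeneralRules, and a debug input zeroes health.
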(event Custom|OnCharacterSelection
  (params (CharacterSelected%20on%20menu :type Personagem%20Generico%20BP%20Class%20Reference))
  ;[1 1 1] É chamado ao selecionar NA THUMBNAIL, apenas seta o personagem
  ; a ser chamado.
  (Variables|Default|SetChar_Selected CharacterSelected%20on%20menu))

(event Custom|RequestServerSpawn
  (params (DestroyedActor :type Actor%20Object%20Reference))
  ;[1 0.1638 0.124] Respawn
  ;;[1 1 1] Ativa o respawn ao detectar que o personagem morreu (no bind event), apenas se o personagem for válido
  (Development|PrintString "Morreu" true true "(R=1.000000,G=0.179376,B=0.000000,A=1.000000)")
  (bind _aspersonagem_generico_bp (Utilities|Casting|CastToPersonagem_Generico_BP DestroyedActor))
  (Utilities|FlowControl|Delay (Variables|/Game/TED_Specific/Character_Assets/Personagem_Generico_BP.Personagem_Generico_BP_C|GetRespawnDelayTime _aspersonagem_generico_bp))
  (Death/Spawn|SequenceRespawnRequest)
  (CallFunction|ResetRespawn))

(event Custom|OnCharacterAccept
  ;[1 1 1] É chamado ao aceitar o personagem selecionado na tela em si e envia o pedido de respawn ao modo de jogo.
  (bind _asgeneral_rules (Utilities|Casting|CastToGeneralRules (Game|GetGameMode)))
  (Default|OnPlayerAcceptSelect _asgeneral_rules self))

(event Custom|ResetRespawn
  ;[1 0.1638 0.124] Respawn
  ;;[1 1 1] Ativa o respawn ao detectar que o personagem morreu (no bind event), apenas se o personagem for válido
  (Utilities|FlowControl|Delay 0.1)
  (Utilities|IsValid (Pawn|GetControlledPawn)
    (:Is%20Valid
      (Game|BindEventtoOnDestroyed (Pawn|GetControlledPawn) (delegate Custom|RequestServerSpawn)))
    (:Is%20Not%20Valid
      (CallFunction|ResetRespawn))))

(event Custom|CallCharRot
  ;[0.2531 0.3765 1] Rotação da câmera
  (if (Utilities|ValidationCharCtrl)
    (if (Utilities|TestVelocity)
      (if (and (Utilities|TestVelocity) (Variables|Default|GetHas_StartedMove))
        (bind _inicharrot (Utilities|CreateCharInitialRot))
        (Variables|Default|SetRot_InitialCharRot _inicharrot)
        (Development|PrintString "Hello")
        (bind _aspersonagem_generico_bp (Utilities|Casting|CastToPersonagem_Generico_BP (Pawn|GetControlledPawn)))
        (bind _rot_alpha (Timeline|Timeline_0 PlayFromStart)
          (:Update
            (if (Utilities|ValidationCharCtrl)
              (Pawn|SetControlRotation (Math|Rotator|Lerp(Rotator) (Variables|Default|GetRot_InitialCharRot) (Variables|/Script/Engine.SceneComponent|GetRelativeRotation (Variables|/Game/TED_Specific/Character_Assets/Personagem_Generico_BP.Personagem_Generico_BP_C|GetSpringArm _aspersonagem_generico_bp)) _rot_alpha true))
              (Variables|Default|SetHas_StartedMove false)))))
      (else
        (Variables|Default|SetHas_StartedMove true)))))

(event EventTick
  (params (DeltaSeconds :type Float%20%28single-precision%29))
  ;[1 1 1] Eventos chamados a todo
  ; momento
  (CallFunction|CallCharRot))

(event EventBeginPlay
  ;[1 0.1638 0.124] Respawn
  (CallFunction|ResetRespawn))

(event Input|ActionEvents|InputActionBotaoTeste
  (params (Key :type Key%20Structure :default "AnyKey"))
  ;[1 1 1] Debug
  (:Pressed
    (bind _aspersonagem_generico_bp (Utilities|Casting|CastToPersonagem_Generico_BP (Pawn|GetControlledPawn)))
    (Variables|/Game/TED_Specific/Character_Assets/Personagem_Generico_BP.Personagem_Generico_BP_C|SetCurHealth _aspersonagem_generico_bp 0)))

(fn ConstructionScript)

(fn ControllerDeathBehavior
  (Pawn|UnPossess)
  (bind _asgeneral_rules (Utilities|Casting|CastToGeneralRules (Game|GetGameMode)))
  (Default|RequestRespawn _asgeneral_rules))

(fn SequenceRespawnRequest
  ;[1 0.1638 0.124] Sequencia de comandos para requisitar o respawn ao modo de jogo
  (bind _asgeneral_rules (Utilities|Casting|CastToGeneralRules (Game|GetGameMode))
    (:then
      (bind _new_char (Default|RequestRespawn _asgeneral_rules (Variables|Default|GetChar_Selected)))
      (Pawn|Possess _new_char))
    (:CastFailed
      (Development|PrintString "CastFail")))
  (return))